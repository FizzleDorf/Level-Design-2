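; Proximity door Blueprint with left and right door parts that open when a Player-tagged actor approaches and close when it leaves.
; On ProximityBox begin overlap, both doors play their animations forward and CollisionBox collision is disabled to clear the way.
; On end overlap, both play at a slower negative rate to reverse, and CollisionBox collision is restored immediately, without waiting for the animation to finish.
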(event `self.ProximityBox.OnComponentBeginOverlap`
  (params (OverlappedComponent :type "PrimitiveComponent Object Reference") (OtherActor :type "Actor Object Reference") (OtherComp :type "PrimitiveComponent Object Reference") (OtherBodyIndex :type Integer) (bFromSweep :type Boolean) (SweepResult :type "HitResult Structure (by ref)"))
  (bind _door_rightdoor (`self.Door_RightDoor`))
  (bind _door_leftdoor (`self.Door_LeftDoor`))
  (if (`self.ActorHasTag` OtherActor "Player")
    (`SkeletalMeshComponent.SetPlayRate` _door_rightdoor 2.5)
    (`SkeletalMeshComponent.Play` _door_rightdoor false)
    (`SkeletalMeshComponent.SetPlayRate` _door_leftdoor 2.5)
    (`SkeletalMeshComponent.Play` _door_leftdoor false)
    (`PrimitiveComponent.SetCollisionEnabled` (`self.CollisionBox`) "NoCollision")))

(event `self.ProximityBox.OnComponentEndOverlap`
  (params (OverlappedComponent :type "PrimitiveComponent Object Reference") (OtherActor :type "Actor Object Reference") (OtherComp :type "PrimitiveComponent Object Reference") (OtherBodyIndex :type Integer))
  (bind _door_leftdoor (`self.Door_LeftDoor`))
  (bind _door_rightdoor (`self.Door_RightDoor`))
  (if (`self.ActorHasTag` OtherActor "Player")
    (`SkeletalMeshComponent.SetPlayRate` _door_leftdoor -2.0)
    (`SkeletalMeshComponent.Play` _door_leftdoor false)
    (`SkeletalMeshComponent.SetPlayRate` _door_rightdoor -2.0)
    (`SkeletalMeshComponent.Play` _door_rightdoor false)
    (`PrimitiveComponent.SetCollisionEnabled` (`self.CollisionBox`) "QueryAndPhysics")))

(fn `UserConstructionScript`)