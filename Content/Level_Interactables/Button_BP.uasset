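; Button_BP is an interactable button that the player activates by overlapping its collision component.
; An overlap from an actor tagged Player sets IsActivated and swaps the static mesh to the Activated material.
; When ShouldReset is set, Tick runs a ResetTime Delay that clears the flag and restores the Inactive material.
; That Delay repeats regardless of activation, so the reset is not timed from the press.
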(event `self.ReceiveTick`
  (params (DeltaSeconds :type "Float (single-precision)"))
  (if (`self.ShouldReset`)
    (`KismetSystemLibrary.Delay` (`self.ResetTime`))
    (set `self.IsActivated` false)
    (`PrimitiveComponent.SetMaterial` (`self.StaticMesh`) 0 "/Game/FirstPerson/Meshes/Inactive.Inactive")))

(event `self.CollisionComponent.OnComponentBeginOverlap`
  (params (OverlappedComponent :type "PrimitiveComponent Object Reference") (OtherActor :type "Actor Object Reference") (OtherComp :type "PrimitiveComponent Object Reference") (OtherBodyIndex :type Integer) (bFromSweep :type Boolean) (SweepResult :type "HitResult Structure (by ref)"))
  (if (`self.ActorHasTag` OtherActor "Player")
    (if (not (`self.IsActivated`))
      (set `self.IsActivated` true)
      (`PrimitiveComponent.SetMaterial` (`self.StaticMesh`) 0 "/Game/FirstPerson/Meshes/Activated.Activated"))))

(fn `UserConstructionScript`)