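; AI smart nav link Blueprint that makes characters jump to the link's destination when they reach it.
; SmartLinkReached casts the agent to a Character and launches it, overriding its current velocity on all axes.
; CalculateVelocity derives the launch velocity from start, destination and JumpDuration, using a projectile-motion formula that compensates for the Gravity variable on Z.
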(event `self.ReceiveSmartLinkReached`
  (params (Agent :type "Actor Object Reference") (Destination :type "Vector Structure (by ref)"))
  (bind _ascharacter (cast `Character` Agent))
  (bind _velocity (`self.CalculateVelocity` Destination (`self.K2_GetActorLocation` _ascharacter) (`self.JumpDuration`)))
  (`Character.LaunchCharacter` _ascharacter _velocity true true))

(fn `CalculateVelocity`
  (params (DestinationLocation :type "Vector Structure") (StartingLocation :type "Vector Structure") (Duration :type "Float (double-precision)"))
  (returns (Velocity :type "Vector Structure"))
  (locals (InDuration :type "Float (double-precision)"))
  (bind _output_get (set `local.InDuration` Duration))
  (return (`KismetMathLibrary.MakeVector` (/ (- DestinationLocation_X StartingLocation_X) _output_get) (/ (- DestinationLocation_Y StartingLocation_Y) _output_get) (/ (- DestinationLocation_Z (+ StartingLocation_Z (* (`KismetMathLibrary.Square` (`local.InDuration`)) -0.5 (`self.Gravity`)))) _output_get))))

(fn `UserConstructionScript`)